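; Inventory component that holds 12 item slots, creates the WPB_Inventory widget on BeginPlay and feeds itself to it.
; IA_OpenPhone toggles the widget along with the mouse cursor and input mode.
; IA_TakeObject sphere-traces around the player's lower body for a BP_Heal, the only supported pickup.
; The item merges into a matching stackable slot capped at quantity 1 or fills an empty one, then the UI reloads and the actor is destroyed.
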(event `EnhancedInput|/Game/ThirdPerson/Input/Actions/IA_OpenPhone`
  (params (ActionValue :type Boolean) (ElapsedSeconds :type "Float (double-precision)") (TriggeredSeconds :type "Float (double-precision)") (InputAction :type "InputAction Object Reference" :default "/Game/ThirdPerson/Input/Actions/IA_OpenPhone.IA_OpenPhone"))
  (bind _returnvalue (`GameplayStatics.GetPlayerController` 0))
  (bind _returnvalue_2 (`GameplayStatics.GetPlayerController` 0))
  (bind _inventorywidget (`self.InventoryWidget`))
  ;[0 0 0] Open
  (:`Started`
    (if (`Widget.IsVisible` (`self.InventoryWidget`))
      (`Widget.RemoveFromParent` _inventorywidget)
      (set `PlayerController.bShowMouseCursor` false _returnvalue_2)
      (`WidgetBlueprintLibrary.SetInputMode_GameOnly` _returnvalue_2)
      (else
        (set `PlayerController.bShowMouseCursor` true _returnvalue)
        (`WidgetBlueprintLibrary.SetInputMode_GameAndUIEx` _returnvalue null)
        (`UserWidget.AddToViewport` _inventorywidget 0)))))

(event `self.ReceiveBeginPlay`
  ;[0 0 0] Loading Inventory & Widget
  (bind _returnvalue (`|CreateWidget` "/Game/Errata/Inventory/WPB_Inventory.WPB_Inventory_C"))
  (set `self.InventoryWidget` _returnvalue)
  (`KismetArrayLibrary.Array_Resize` (`self.Items`) 12)
  (`/Game/Errata/Inventory/WPB_Inventory.LoadInventory` (`self.InventoryWidget`) self))

(event `EnhancedInput|/Game/ThirdPerson/Input/Actions/IA_TakeObject`
  (params (ActionValue :type Boolean) (ElapsedSeconds :type "Float (double-precision)") (TriggeredSeconds :type "Float (double-precision)") (InputAction :type "InputAction Object Reference" :default "/Game/ThirdPerson/Input/Actions/IA_TakeObject.IA_TakeObject"))
  (bind _returnvalue (- (`Actor.K2_GetActorLocation` (`GameplayStatics.GetPlayerCharacter` 0)) (0.0 0.0 65.0)))
  ;[0 0 0] To add item to inventory
  (:`Started`
    (bind _outhit (`KismetSystemLibrary.SphereTraceSingle` _returnvalue _returnvalue 120.0 "TraceTypeQuery1"))
    ;[0 0 0] Update inventory UI
    (bind _asbp_heal (cast `/Game/Errata/Blueprints/BP_Heal` (`.HitActor` (`GameplayStatics.BreakHitResult` _outhit))))
    (for (_array_element _array_index) (`self.Items`)
      (`/Engine/EditorBlueprintResources/StandardMacros.IsValid` _asbp_heal
        (:`Is Valid`
          (bind (_name _stackable _quantity) (break `/Game/Errata/Inventory/BPS_ItemStructure` _array_element))
          (bind (_name_2 _stackable_2 _quantity_2) (break `/Game/Errata/Inventory/BPS_ItemStructure` (`/Game/Errata/Blueprints/BP_Heal.Item` _asbp_heal)))
          (bind _returnvalue_2 (+ _quantity _quantity_2))
          (if (and (`KismetTextLibrary.EqualEqual_TextText` _name _name_2) _stackable_2 (<= _returnvalue_2 1))
            (bind (_item_name _item_stackable _item_quantity _item_thumbnail _item_mesh) (break `/Game/Errata/Inventory/BPS_ItemStructure` (`/Game/Errata/Blueprints/BP_Heal.Item` _asbp_heal)))
            (`KismetArrayLibrary.Array_Set` (`self.Items`) _array_index (make `/Game/Errata/Inventory/BPS_ItemStructure` _item_name _item_stackable _returnvalue_2 _item_thumbnail _item_mesh))
            (`/Game/Errata/Inventory/WPB_Inventory.LoadInventory` (`self.InventoryWidget`) self :!label _label)
            (`KismetSystemLibrary.PrintString` "Heal Taken")
            (`Actor.K2_DestroyActor` _asbp_heal)
            (`KismetSystemLibrary.PrintString` "Heal Destroyed")
            (elif (== _quantity 0)
              (`KismetArrayLibrary.Array_Set` (`self.Items`) _array_index (`/Game/Errata/Blueprints/BP_Heal.Item` _asbp_heal))
              (goto _label))))))))