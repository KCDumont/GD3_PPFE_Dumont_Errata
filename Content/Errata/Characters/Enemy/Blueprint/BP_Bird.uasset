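; Bird enemy character that chases and attacks the player in a third-person game.
; Pawn sensing starts an AI move to the player, then a random attack montage damages Mallory directly; its line trace result is unused.
; Hits reduce health with random reactions; damage received at zero health or below plays death, notifies the game mode and destroys the bird.
; A sphere overlap toggles a distortion sound.
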(event `self.ReceiveBeginPlay`
  (`KismetSystemLibrary.Delay` 1.0)
  (bind _returnvalue (`GameplayStatics.GetActorOfClass` "/Game/ThirdPerson/Blueprints/BP_ThirdPersonCharacter.BP_ThirdPersonCharacter_C"))
  (set `self.Mallory` _returnvalue)
  (bind _asbp_third_person_game_mode (cast `/Game/ThirdPerson/Blueprints/BP_ThirdPersonGameMode` (`GameplayStatics.GetGameMode`)))
  (set `self.Game Mode Ref` _asbp_third_person_game_mode))

(event `Bird Attack`
  (bind _attackanims (`self.AttackAnims`))
  (bind _returnvalue (`SceneComponent.GetSocketLocation` (`self.Attack`) "None"))
  ;[0 0 0] Bird Attack
  (`CharacterMovementComponent.SetMovementMode` (`self.CharacterMovement`) "MOVE_None" 0)
  (`self.PlayAnimMontage` (`|GetArrayItem` _attackanims (`KismetMathLibrary.RandomInteger` (`KismetArrayLibrary.Array_Length` _attackanims))) 0.5)
  (`KismetSystemLibrary.LineTraceSingle` _returnvalue _returnvalue "TraceTypeQuery1")
  (`/Game/ThirdPerson/Blueprints/BP_ThirdPersonCharacter.TakeDamage` (`self.Mallory`) 10.0)
  (`KismetSystemLibrary.Delay` 5.0)
  (set `self.CanAttack` true)
  (`CharacterMovementComponent.SetMovementMode` (`self.CharacterMovement`) "MOVE_Walking" 0))

(event `self.PawnSensing.OnSeePawn`
  (params (Pawn :type "Pawn Object Reference"))
  ;[0 0 0] Follow Player
  (set `self.isSeeingMallory?` true)
  (`self.FollowPlayer`))

(event `FollowPlayer`
  ;[0 0 0] Follow Player
  (if (`self.isSeeingMallory?`)
    (set `self.CanAttack` true)
    (`|AIMoveTo` self (0.0 0.0 0.0) (`GameplayStatics.GetPlayerCharacter` 0) 25.0
      (:`OnSuccess`
        ;[0 0 0] Calling Attack
        (if (`self.CanAttack`)
          (`self.Bird Attack`))))
    (else
      (set `self.isSeeingMallory?` false))))

(event `self.ReceiveAnyDamage`
  (params (Damage :type "Float (single-precision)") (DamageType :type "DamageType Object Reference") (InstigatedBy :type "Controller Object Reference") (DamageCauser :type "Actor Object Reference"))
  (bind _takehitanims (`self.TakeHitAnims`))
  ;[0 0 0] Taking Damage
  (if (> (`self.Health`) 0.0)
    (set `self.Health` (- (`self.Health`) Damage))
    (`CharacterMovementComponent.SetMovementMode` (`self.CharacterMovement`) "MOVE_None" 0)
    (`self.PlayAnimMontage` (`|GetArrayItem` _takehitanims (`KismetMathLibrary.RandomInteger` (`KismetArrayLibrary.Array_Length` _takehitanims))))
    (`GameplayStatics.PlaySound2D` "/Game/Errata/SoundDesign/SoundEffects/Mallory/SEC_Attack.SEC_Attack" 1.0 1.0 0.0 null null)
    (else
      (`CharacterMovementComponent.DisableMovement` (`self.CharacterMovement`))
      (`GameplayStatics.SpawnSound2D` "/Game/Errata/SoundDesign/SoundEffects/Bird/SE_BirdDying.SE_BirdDying" 1.0 1.0 0.0 null)
      (`self.PlayAnimMontage` "/Game/Errata/Characters/Enemy/Anims/AM_Bird_Dying.AM_Bird_Dying")
      (`/Game/ThirdPerson/Blueprints/BP_ThirdPersonGameMode.EnnemiesDied` (`self.Game Mode Ref`) self)
      (`KismetSystemLibrary.Delay` 2.0)
      (`self.K2_DestroyActor`))))

(event `self.Sphere.OnComponentBeginOverlap`
  (params (OverlappedComponent :type "PrimitiveComponent Object Reference") (OtherActor :type "Actor Object Reference") (OtherComp :type "PrimitiveComponent Object Reference") (OtherBodyIndex :type Integer) (bFromSweep :type Boolean) (SweepResult :type "HitResult Structure (by ref)"))
  ;[0 0 0] Bird Distortion
  (`AudioComponent.Play` (`self.SEC_BirdDistortion`) 0.0))

(event `self.Sphere.OnComponentEndOverlap`
  (params (OverlappedComponent :type "PrimitiveComponent Object Reference") (OtherActor :type "Actor Object Reference") (OtherComp :type "PrimitiveComponent Object Reference") (OtherBodyIndex :type Integer))
  ;[0 0 0] Bird Distortion
  (`AudioComponent.Stop` (`self.SEC_BirdDistortion`)))

(fn `UserConstructionScript`)