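; BP_StagKing is the Stag King enemy that hunts the player character Mallory, replacing the ambient music with its own sound on BeginPlay.
; Pawn sensing triggers an AI move to the player, then an attack that pauses movement, plays a random montage and damages Mallory regardless of its line trace.
; Incoming damage lowers Health with random hit reactions or plays a death montage at zero, though this path is marked not working.
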(event `self.ReceiveBeginPlay`
  (bind _returnvalue (`GameplayStatics.GetActorOfClass` "/Game/ThirdPerson/Blueprints/BP_ThirdPersonCharacter.BP_ThirdPersonCharacter_C"))
  (bind _output_get (set `self.Mallory` _returnvalue))
  (`AudioComponent.Stop` (`/Game/ThirdPerson/Blueprints/BP_ThirdPersonCharacter.AmbiantMusic` _output_get))
  (`GameplayStatics.SpawnSound2D` "/Game/Errata/SoundDesign/Music/SDC_StagKing.SDC_StagKing" 1.0 1.0 0.0 null))

(event `Stag King Attack`
  (bind _attackanims (`self.AttackAnims`))
  (bind _returnvalue (`SceneComponent.GetSocketLocation` (`self.Attack`) "None"))
  ;[0 0 0] Stag King Attack
  (`CharacterMovementComponent.SetMovementMode` (`self.CharacterMovement`) "MOVE_None" 0)
  (`self.PlayAnimMontage` (`|GetArrayItem` _attackanims (`KismetMathLibrary.RandomInteger` (`KismetArrayLibrary.Array_Length` _attackanims))))
  (`KismetSystemLibrary.LineTraceSingle` _returnvalue _returnvalue "TraceTypeQuery1")
  (`/Game/ThirdPerson/Blueprints/BP_ThirdPersonCharacter.TakeDamage` (`self.Mallory`) 5.0)
  (`KismetSystemLibrary.Delay` 1.0)
  (set `self.CanSKAttack?` true)
  (`CharacterMovementComponent.SetMovementMode` (`self.CharacterMovement`) "MOVE_Walking" 0))

(event `self.SensingMallory.OnSeePawn`
  (params (Pawn :type "Pawn Object Reference"))
  ;[0 0 0] Follow Mallory
  (set `self.IsSeeingMallory?` true)
  (`self.FollowMallory`))

(event `FollowMallory`
  ;[0 0 0] Follow and Attack Mallory
  (if (`self.IsSeeingMallory?`)
    (set `self.CanSKAttack?` true)
    (`|AIMoveTo` self (0.0 0.0 0.0) (`GameplayStatics.GetPlayerCharacter` 0) 10.0
      (:`OnSuccess`
        (if (`self.CanSKAttack?`)
          (`self.Stag King Attack`))))
    (else
      (set `self.IsSeeingMallory?` false))))

(event `self.ReceiveAnyDamage`
  (params (Damage :type "Float (single-precision)") (DamageType :type "DamageType Object Reference") (InstigatedBy :type "Controller Object Reference") (DamageCauser :type "Actor Object Reference"))
  (bind _takehitanims (`self.TakeHitAnims`))
  ;[0.2031 0 0] Taking Damage NOT WORKING
  (if (> (`self.Health`) 0.0)
    (set `self.Health` (- (`self.Health`) Damage))
    (`self.PlayAnimMontage` (`|GetArrayItem` _takehitanims (`KismetMathLibrary.RandomInteger` (`KismetArrayLibrary.Array_Length` _takehitanims))))
    (else
      (`self.PlayAnimMontage` "/Game/Errata/Characters/StagKing/Anims/AM_SK_Dying.AM_SK_Dying"))))

(fn `UserConstructionScript`)